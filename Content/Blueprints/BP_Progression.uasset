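; BP_Progression loads the player's saved progression: double jump unlock, completed levels and collected stars.
; On Init it reads a BP_SavedProgression from the save slot, or creates a fresh one when none exists.
; Levels and stars are copied only if jump is unlocked.
; The star loop is nested inside the level loop, so stars need at least one completed level and rely on AddUnique against duplicates.
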(event EventInit
  (bind _returnvalue (SaveGame|DoesSaveGameExist (Variables|Default|GetSaveSlot)))
  (if _returnvalue
    (bind _returnvalue_2 (SaveGame|LoadGamefromSlot (Variables|Default|GetSaveSlot)))
    (bind _asbp_saved_progression (Utilities|Casting|CastToBP_SavedProgression _returnvalue_2))
    (bind _output_get (Variables|Default|SetSavedGameData _asbp_saved_progression))
    (if (Variables|/Game/Blueprints/BP_SavedProgression.BP_SavedProgression_C|GetbJumpUnlocked _output_get)
      (Variables|Default|SetbPlayerDoubleJump true)
      (for _array_element (Variables|/Game/Blueprints/BP_SavedProgression.BP_SavedProgression_C|GetLevelcomplete (Variables|Default|GetSavedGameData))
        (Utilities|Array|Add (Variables|Default|GetLevelsComplete) _array_element)
        (for _array_element_2 (Variables|/Game/Blueprints/BP_SavedProgression.BP_SavedProgression_C|GetCollectedStars (Variables|Default|GetSavedGameData))
          (Utilities|Array|AddUnique (Variables|Default|GetCollectedStars) _array_element_2))))
    (else
      (bind _returnvalue_3 (SaveGame|CreateSaveGameObject "/Game/Blueprints/BP_SavedProgression.BP_SavedProgression_C"))
      (Variables|Default|SetSavedGameData _returnvalue_3))))