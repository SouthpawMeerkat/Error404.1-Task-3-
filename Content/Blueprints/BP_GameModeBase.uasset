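; Base game mode that owns the game's UI: menus, player HUD and death screen.
; BeginPlay creates and caches every widget up front, and MenuRunner clears all widgets, then shows the menu matching CurrentMenu.
; HealthChanger and ScoreChanger forward values to the player HUD, while LevelSetUp switches to game-only input and hides the cursor.
; The HUD and death screen are never added to the viewport here.
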(event EventBeginPlay
  (CallFunction|MenuSetUp))

(fn ConstructionScript)

(fn MenuSetUp
  (bind _returnvalue (UserInterface|CreateWidget "/Game/Blueprints/UI/MainMenu.MainMenu_C"))
  (Variables|Default|SetMainMenuRef _returnvalue)
  (bind _returnvalue_2 (UserInterface|CreateWidget "/Game/Blueprints/UI/LevelMenu.LevelMenu_C"))
  (Variables|Default|SetLevelMenuRef _returnvalue_2)
  (bind _returnvalue_3 (UserInterface|CreateWidget "/Game/Blueprints/UI/SettingMenu.SettingMenu_C"))
  (Variables|Default|SetSettingsMenuRef _returnvalue_3)
  (bind _returnvalue_4 (UserInterface|CreateWidget "/Game/Blueprints/UI/AchievmentsMenu.AchievmentsMenu_C"))
  (Variables|Default|SetAchievmentMenuRef _returnvalue_4)
  (bind _returnvalue_5 (UserInterface|CreateWidget "/Game/Blueprints/UI/CharacterMenu.CharacterMenu_C"))
  (Variables|Default|SetCharacterMenuRef _returnvalue_5)
  (bind _returnvalue_6 (UserInterface|CreateWidget "/Game/Blueprints/UI/PlayerUI.PlayerUI_C"))
  (Variables|Default|SetPlayerInfoUIRef _returnvalue_6)
  (bind _returnvalue_7 (UserInterface|CreateWidget "/Game/Blueprints/UI/DeathScreen.DeathScreen_C"))
  (Variables|Default|SetDeathScreenRef _returnvalue_7))

(fn LevelSetUp
  (bind _returnvalue (Game|GetPlayerController 0))
  (Input|SetInputModeGameOnly _returnvalue false)
  (Variables|/Script/Engine.PlayerController|SetbShowMouseCursor _returnvalue false))

(fn MenuRunner
  (Viewport|RemoveAllWidgets)
  (switch string (Variables|Default|GetCurrentMenu)
    (:Main
      (UserInterface|Viewport|AddtoViewport (Variables|Default|GetMainMenuRef) 0))
    (:Level
      (UserInterface|Viewport|AddtoViewport (Variables|Default|GetLevelMenuRef) 0))
    (:Achievement
      (UserInterface|Viewport|AddtoViewport (Variables|Default|GetAchievmentMenuRef) 0))
    (:Character
      (UserInterface|Viewport|AddtoViewport (Variables|Default|GetCharacterMenuRef) 0))
    (:Setting
      (UserInterface|Viewport|AddtoViewport (Variables|Default|GetSettingsMenuRef) 0))))

(fn HealthChanger
  (params (Health :type Float%20%28double-precision%29) (MaxHealth :type Float%20%28double-precision%29))
  (Default|UpdateHealth (Variables|Default|GetPlayerInfoUIRef) Health MaxHealth))

(fn ScoreChanger
  (params (New%20Score :type Integer))
  (Default|UpdateScoreText (Variables|Default|GetPlayerInfoUIRef) New%20Score))