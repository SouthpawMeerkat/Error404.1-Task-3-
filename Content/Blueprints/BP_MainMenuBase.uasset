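; Main menu controller Blueprint that owns the game's menu screens and switches between them.
; On BeginPlay it sets UI-only input with a visible cursor, creates and caches the main, level, settings, achievements and character widgets, then shows the main menu.
; MenuRunner removes all widgets and adds the cached one matching CurrentMenu to the viewport; that variable is set outside these graphs.
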(event EventBeginPlay
  (bind _returnvalue (Game|GetPlayerController 0))
  (Input|SetInputModeUIOnly _returnvalue 0 "DoNotLock" false)
  (Variables|/Script/Engine.PlayerController|SetbShowMouseCursor _returnvalue true)
  (bind _returnvalue_2 (UserInterface|CreateWidget "/Game/Blueprints/UI/MainMenu.MainMenu_C"))
  (Variables|Default|SetMainMenuRef _returnvalue_2)
  (bind _returnvalue_3 (UserInterface|CreateWidget "/Game/Blueprints/UI/LevelMenu.LevelMenu_C"))
  (Variables|Default|SetLevelMenuRef _returnvalue_3)
  (bind _returnvalue_4 (UserInterface|CreateWidget "/Game/Blueprints/UI/SettingMenu.SettingMenu_C"))
  (Variables|Default|SetSettingsMenuRef _returnvalue_4)
  (bind _returnvalue_5 (UserInterface|CreateWidget "/Game/Blueprints/UI/AchievmentsMenu.AchievmentsMenu_C"))
  (Variables|Default|SetAchievmentMenuRef _returnvalue_5)
  (bind _returnvalue_6 (UserInterface|CreateWidget "/Game/Blueprints/UI/CharacterMenu.CharacterMenu_C"))
  (Variables|Default|SetCharacterMenuRef _returnvalue_6)
  (UserInterface|Viewport|AddtoViewport (Variables|Default|GetMainMenuRef) 0))

(fn ConstructionScript)

(fn MenuRunner
  (Viewport|RemoveAllWidgets)
  (switch string (Variables|Default|GetCurrentMenu)
    (:Main
      (UserInterface|Viewport|AddtoViewport (Variables|Default|GetMainMenuRef) 0))
    (:Level
      (UserInterface|Viewport|AddtoViewport (Variables|Default|GetLevelMenuRef) 0))
    (:Achievement
      (UserInterface|Viewport|AddtoViewport (Variables|Default|GetAchievmentMenuRef) 0))
    (:Character
      (UserInterface|Viewport|AddtoViewport (Variables|Default|GetCharacterMenuRef) 0))
    (:Setting
      (UserInterface|Viewport|AddtoViewport (Variables|Default|GetSettingsMenuRef) 0))))