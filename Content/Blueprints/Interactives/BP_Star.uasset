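; Collectible star that registers with BP_GameModeBase's level star count and persists its pickup, identified by the flipbook's world location.
; Interact adds that location to BP_Progression's SavedGameData, saves the slot, updates the game mode's collected list and counter, then destroys the star.
; BeginPlay checks BP_Progression's own CollectedStars, not SavedGameData, and on a location match marks the star collected, plays a sound and destroys it.
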(event EventBeginPlay
  (bind _asbp_game_mode_base (Utilities|Casting|CastToBP_GameModeBase (Game|GetGameMode)))
  (Utilities|Array|Add (Variables|/Game/Blueprints/BP_GameModeBase.BP_GameModeBase_C|GetLevelStarCount _asbp_game_mode_base) self)
  (Default|CollectableChanger _asbp_game_mode_base)
  (bind _asbp_progression (Utilities|Casting|CastToBP_Progression (Game|GetGameInstance)))
  (for _array_element (Variables|/Game/Blueprints/BP_Progression.BP_Progression_C|GetCollectedStars _asbp_progression)
    (if (Utilities|Operators|EqualEqual (Transformation|GetWorldLocation (Variables|Default|GetPaperFlipbook)) _array_element 1.0)
      (bind _asbp_game_mode_base_2 (Utilities|Casting|CastToBP_GameModeBase (Game|GetGameMode)))
      (Utilities|Array|AddUnique (Variables|/Game/Blueprints/BP_GameModeBase.BP_GameModeBase_C|GetLevelStarsCollected _asbp_game_mode_base_2) (Transformation|GetWorldLocation (Variables|Default|GetPaperFlipbook)))
      (Audio|PlaySound2D "/Game/Assets/Sounds/BlueStar_collectible.BlueStar_collectible" 1.0 1.0 0.0 0 0)
      (Actor|DestroyActor)
      (Default|CollectableChanger _asbp_game_mode_base_2))))

(fn ConstructionScript
  (|CallParentFunction))

(fn Interact
  (params (PlayerRef :type BP%20Player%20Base%20Object%20Reference))
  (bind _asbp_progression (Utilities|Casting|CastToBP_Progression (Game|GetGameInstance)))
  (Utilities|Array|AddUnique (Variables|/Game/Blueprints/BP_SavedProgression.BP_SavedProgression_C|GetCollectedStars (Variables|/Game/Blueprints/BP_Progression.BP_Progression_C|GetSavedGameData _asbp_progression)) (Transformation|GetWorldLocation (Variables|Default|GetPaperFlipbook)))
  (SaveGame|SaveGametoSlot (Variables|/Game/Blueprints/BP_Progression.BP_Progression_C|GetSavedGameData _asbp_progression) (Variables|/Game/Blueprints/BP_Progression.BP_Progression_C|GetSaveSlot _asbp_progression))
  (bind _asbp_game_mode_base (Utilities|Casting|CastToBP_GameModeBase (Game|GetGameMode)))
  (Utilities|Array|AddUnique (Variables|/Game/Blueprints/BP_GameModeBase.BP_GameModeBase_C|GetLevelStarsCollected _asbp_game_mode_base) (Transformation|GetWorldLocation (Variables|Default|GetPaperFlipbook)))
  (Actor|DestroyActor)
  (Default|CollectableChanger _asbp_game_mode_base))