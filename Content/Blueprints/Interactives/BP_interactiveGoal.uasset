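; BP_interactiveGoal is an interactive goal actor that shows the win screen when the player interacts with it.
; Interact switches input to UI only, shows the mouse cursor, clears all widgets and adds a new WinScreen to the viewport.
; Separately, any actor overlap while Unlock is true sets PlayerDoubleJump on the BP_Progression game instance, granting double jump.
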(event Collision|EventActorBeginOverlap
  (params (OtherActor :type Actor%20Object%20Reference))
  (if (Variables|Default|GetUnlock)
    (bind _asbp_progression (Utilities|Casting|CastToBP_Progression (Game|GetGameInstance)))
    (Variables|/Game/Blueprints/BP_Progression.BP_Progression_C|SetbPlayerDoubleJump _asbp_progression true)))

(fn ConstructionScript
  (|CallParentFunction))

(fn Interact
  (params (PlayerRef :type BP%20Player%20Base%20Object%20Reference))
  (bind _returnvalue (Game|GetPlayerController 0))
  (Input|SetInputModeUIOnly _returnvalue 0 "DoNotLock" false)
  (Variables|/Script/Engine.PlayerController|SetbShowMouseCursor _returnvalue true)
  (Viewport|RemoveAllWidgets)
  (bind _returnvalue_2 (UserInterface|CreateWidget "/Game/Blueprints/UI/WinScreen.WinScreen_C"))
  (UserInterface|Viewport|AddtoViewport _returnvalue_2 0))