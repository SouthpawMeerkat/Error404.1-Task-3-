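; Slime enemy that shoots slime balls at the player when within range and destroys itself on death.
; Tick checks player distance; a Delay throttles attacks, then switches to the monster flipbook and spawns BP_SlimeBall rotated toward the player's capsule.
; Out of range it shows the idle flipbook, though a pending Delay still fires.
; EnemyDied calls the parent logic before destroying the actor.
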(event EventTick
  (params (DeltaSeconds :type Float%20%28single-precision%29))
  (if (<= (Transformation|GetDistanceTo (Game|GetPlayerCharacter 0)) 1e+03)
    (Utilities|FlowControl|Delay 1.5)
    (Sprite|SetFlipbook (Variables|Default|GetSprite) "/Game/Assets/FlipBook/FB_monster.FB_monster")
    (Game|SpawnActorfromClass "/Game/Blueprints/Enemies/BP_SlimeBall.BP_SlimeBall_C" (Math|Transform|MakeTransform (Transformation|GetWorldLocation (Variables|Default|GetCapsuleComponent)) (Math|Rotator|FindLookatRotation (Transformation|GetWorldLocation (Variables|Default|GetCapsuleComponent)) (Transformation|GetWorldLocation (Variables|/Script/Engine.Character|GetCapsuleComponent (Game|GetPlayerCharacter 0)))) "1.000000,1.000000,1.000000") "Undefined" "MultiplyWithRoot" 0 0)
    (else
      (Sprite|SetFlipbook (Variables|Default|GetSprite) "/Game/Assets/FlipBook/FB_monsterIdle.FB_monsterIdle"))))

(fn ConstructionScript
  (|CallParentFunction))

(fn EnemyDied
  (|CallParentFunction)
  (Actor|DestroyActor))